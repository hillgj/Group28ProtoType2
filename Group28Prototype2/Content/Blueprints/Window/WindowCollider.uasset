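; Window trigger volume that toggles a reactor camera view message on the first player's controller.
; Begin and end overlap on Collider check that the other actor is owned by player controller 0, then call ToggleViewMessage on or off with the ReactorCamera reference.
; StartReactorCamera and EndReactorCamera events run the same logic directly and track ChangedPerspective.
; The Overlapping flag follows overlaps from any actor, as it is set before the owner check.
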(event OnComponentBeginOverlap(Collider)
  (params (OverlappedComponent :type Primitive%20Component%20Object%20Reference) (OtherActor :type Actor%20Object%20Reference) (OtherComp :type Primitive%20Component%20Object%20Reference) (OtherBodyIndex :type Integer) (bFromSweep :type Boolean) (SweepResult :type Hit%20Result%20Structure%20%28by%20ref%29))
  (Variables|Default|Set%20Overlapping true)
  (if (== (Components|GetOwner OtherActor) (Game|GetPlayerController 0))
    (Class|ActivateWindowView|ToggleView(Message) (Game|GetPlayerController 0) true (Variables|Default|GetReactorCamera))
    (Variables|Default|SetChangedPerspective true)))

(event OnComponentEndOverlap(Collider)
  (params (OverlappedComponent :type Primitive%20Component%20Object%20Reference) (OtherActor :type Actor%20Object%20Reference) (OtherComp :type Primitive%20Component%20Object%20Reference) (OtherBodyIndex :type Integer))
  (Variables|Default|Set%20Overlapping false)
  (if (== (Components|GetOwner OtherActor) (Game|GetPlayerController 0))
    (Class|ActivateWindowView|ToggleView(Message) (Game|GetPlayerController 0) false (Variables|Default|GetReactorCamera))
    (Variables|Default|SetChangedPerspective false)))

(event Custom|StartReactorCamera
  (Class|ActivateWindowView|ToggleView(Message) (Game|GetPlayerController 0) true (Variables|Default|GetReactorCamera))
  (Variables|Default|SetChangedPerspective true))

(event Custom|EndReactorCamera
  (Class|ActivateWindowView|ToggleView(Message) (Game|GetPlayerController 0) false (Variables|Default|GetReactorCamera))
  (Variables|Default|SetChangedPerspective false))

(fn ConstructionScript)