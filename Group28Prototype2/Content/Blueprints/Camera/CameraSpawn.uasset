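; CameraSpawn is a camera Blueprint that turns to follow the player character.
; Every Tick, it computes a look-at rotation from the camera to the PlayerCharacter mesh and eases the camera toward it with a slow RInterpTo.
; The interpolation uses a constant DeltaTime instead of the frame delta, so the turn speed depends on frame rate.
; The graphs only rotate the camera and never move it.
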(event EventTick
  (params (DeltaSeconds :type Float%20%28single-precision%29))
  (Transformation|SetWorldRotation (Variables|Default|GetCamera) (Math|Interpolation|RInterpTo (Transformation|GetWorldRotation (Variables|Default|GetCamera)) (Math|Rotator|FindLookatRotation (Transformation|GetWorldLocation (Variables|Default|GetCamera)) (Transformation|GetWorldLocation (Variables|/Script/Engine.Character|GetMesh (Variables|Default|GetPlayerCharacter)))) 1.0 0.04) false false))

(fn ConstructionScript
  (Variables|Default|Set_Camera (Variables|Default|GetCamera)))