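; Player controller for two swappable characters in a reactor game, creating the player UI and starting on a tagged lab camera.
; Swapping possesses the other character, restores a stored control rotation and starts or ends the WindowCollider's reactor camera.
; Interact toggles overlapped objects from the GameManager's list, with handlers picked by array index and one shared Interacted flag.
; Arrow keys adjust reactor instability; left-click drives TaskMaster widget pointers.
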(event Custom|SetLabCamera
  (params (Time :type Float%20%28single-precision%29))
  (bind _outactors (Actor|GetAllActorswithTag "Camera"))
  (Game|Player|SetViewTargetwithBlend (.AsCamera%20Spawn (Utilities|Casting|CastToCameraSpawn (Utilities|Array|Get(acopy) _outactors))) Time "VTBlend_EaseInOut" 1.0 true)
  (Variables|Misc|SetCurrentViewTarget (.AsCamera%20Spawn (Utilities|Casting|CastToCameraSpawn (Utilities|Array|Get(acopy) _outactors)))))

(event Custom|PressureInteraction
  (params (Object :type Object%20Object%20Reference))
  (bind _aspressure_monitor (Utilities|Casting|CastToPressureMonitor Object))
  (if (Variables|/Game/Blueprints/ReactorParts/PressureMonitor.PressureMonitor_C|GetOverlapped _aspressure_monitor)
    (if (Variables|Misc|GetInteracted)
      (bind _output_get (Variables|Misc|SetInteracted false))
      (Class|ActivateInteractable|ToggleObject(Message) Object _output_get)
      (else
        (bind _output_get_2 (Variables|Misc|SetInteracted true))
        (Class|ActivateInteractable|ToggleObject(Message) Object _output_get_2)))))

(event Custom|ReactorInteraction
  (params (Reactor :type Actor%20Object%20Reference))
  (bind _asreactor (Utilities|Casting|CastToReactor Reactor))
  (if (Variables|/Game/Blueprints/ReactorParts/Reactor.Reactor_C|GetOverlapped _asreactor)
    (if (Variables|Misc|GetInteracted)
      (bind _output_get (Variables|Misc|SetInteracted false))
      (Class|ActivateInteractable|ToggleObject(Message) Reactor _output_get)
      (else
        (bind _output_get_2 (Variables|Misc|SetInteracted true))
        (Class|ActivateInteractable|ToggleObject(Message) Reactor _output_get_2)))))

(event Custom|PowerInteraction
  (params (Object :type Object%20Object%20Reference))
  (bind _aspower_flow_monitor (Utilities|Casting|CastToPowerFlowMonitor Object))
  (if (Variables|/Game/Blueprints/ReactorParts/PowerFlowMonitor.PowerFlowMonitor_C|GetOverlapped _aspower_flow_monitor)
    (if (Variables|Misc|GetInteracted)
      (bind _output_get (Variables|Misc|SetInteracted false))
      (Class|ActivateInteractable|ToggleObject(Message) Object _output_get)
      (else
        (bind _output_get_2 (Variables|Misc|SetInteracted true))
        (Class|ActivateInteractable|ToggleObject(Message) Object _output_get_2)))))

(event Custom|TempInteraction
  (params (Temp :type Actor%20Object%20Reference))
  (bind _astemp_monitor (Utilities|Casting|CastToTempMonitor Temp))
  (if (Variables|/Game/Blueprints/ReactorParts/TempMonitor.TempMonitor_C|GetOverlapped _astemp_monitor)
    (if (Variables|Misc|GetInteracted)
      (bind _output_get (Variables|Misc|SetInteracted false))
      (Class|ActivateInteractable|ToggleObject(Message) Temp _output_get)
      (else
        (bind _output_get_2 (Variables|Misc|SetInteracted true))
        (Class|ActivateInteractable|ToggleObject(Message) Temp _output_get_2)))))

(event Custom|ExampleInteraction
  (params (Object :type Object%20Object%20Reference))
  (bind _astask_master (Utilities|Casting|CastToTaskMaster Object))
  (if (Variables|/Game/Blueprints/Tasks/TaskMaster/TaskMaster.TaskMaster_C|GetOverlapped _astask_master)
    (if (Variables|Misc|GetInteracted)
      (bind _output_get (Variables|Misc|SetInteracted false))
      (Class|ActivateInteractable|ToggleObject(Message) Object _output_get)
      (else
        (bind _output_get_2 (Variables|Misc|SetInteracted true))
        (Class|ActivateInteractable|ToggleObject(Message) Object _output_get_2)))))

(event EventBeginPlay
  (Variables|Default|SetNewControlRotationP1 (Pawn|GetControlRotation :!class /Script/Engine.Controller))
  (Variables|Default|SetNewControlRotationP2 "0, 0, 0")
  (bind _returnvalue (UserInterface|CreateWidget "/Game/UI/PlayerUI.PlayerUI_C"))
  (UserInterface|Viewport|AddtoViewport _returnvalue 0)
  (bind _outactors (Actor|GetAllActorsOfClasswithTag "/Game/Blueprints/GameManager.GameManager_C" "GM"))
  (Variables|Misc|SetWindowCollider (Variables|/Game/Blueprints/GameManager.GameManager_C|GetWindow%20Collider (Utilities|Array|Get(acopy) _outactors)))
  (Variables|Misc|SetInteractables (Variables|/Game/Blueprints/GameManager.GameManager_C|GetInteractables (Utilities|Array|Get(acopy) _outactors)))
  (CallFunction|SetLabCamera 0.0)
  (bind _outactors_2 (Actor|GetAllActorsOfClass "/Game/Blueprints/Player/Character.Character_C"))
  (for (_array_element _array_index) _outactors_2
    (Utilities|Map|Add (Variables|Misc|GetCharacters) _array_index _array_element)
    (if (== _array_element (Game|Player|GetPlayerPawn 0))
      (Variables|Misc|SetCurrentCharacterIndex _array_index))))

(event EventToggleView
  (params (State :type Boolean) (ReactorCamera :type Window%20Camera%20Object%20Reference))
  (if State
    (Game|Player|SetViewTargetwithBlend ReactorCamera 0.7 "VTBlend_EaseInOut" 1.0 true)
    (Variables|Misc|SetCurrentViewTarget ReactorCamera)
    (else
      (CallFunction|SetLabCamera 0.7))))

(event Input|ActionEvents|InputActionSwapCharacter
  (params (Key :type Key%20Structure :default "None"))
  (bind _windowcollider (Variables|Misc|GetWindowCollider))
  (bind _characters (Variables|Misc|GetCharacters))
  (bind _characters_2 (Variables|Misc|GetCharacters))
  (bind _windowcollider_2 (Variables|Misc|GetWindowCollider))
  (bind (_value _returnvalue) (Utilities|Map|Find _characters 0))
  (bind (_value_2 _returnvalue_2) (Utilities|Map|Find _characters_2 1))
  (:Pressed
    (if (== (.Value (Utilities|Map|Find (Variables|Misc|GetCharacters) 0)) (Game|Player|GetPlayerPawn 0))
      (Variables|Misc|SetCurrentCharacterIndex 1)
      (else
        (Variables|Misc|SetCurrentCharacterIndex 0)))
    (switch int (Variables|Misc|GetCurrentCharacterIndex)
      (:Default
        (Development|PrintString "only 2 characters supported (ask harley for more)"))
      (:0
        (if _returnvalue
          (Pawn|Possess (Game|GetPlayerController 0) _value)
          (Pawn|SetControlRotation (Variables|Default|GetNewControlRotationP1))
          (if (and (not (Variables|/Game/Blueprints/Window/WindowCollider.WindowCollider_C|Get%20Overlapping _windowcollider_2)) (Variables|/Game/Blueprints/Window/WindowCollider.WindowCollider_C|GetChangedPerspective _windowcollider_2))
            (Default|EndReactorCamera _windowcollider_2)
            (Variables|/Game/Blueprints/Window/WindowCollider.WindowCollider_C|SetChangedPerspective _windowcollider_2 false))))
      (:1
        (if _returnvalue_2
          (Pawn|Possess (Game|GetPlayerController 0) _value_2)
          (Pawn|SetControlRotation (Variables|Default|GetNewControlRotationP2))
          (if (not (Variables|/Game/Blueprints/Window/WindowCollider.WindowCollider_C|GetChangedPerspective _windowcollider))
            (Default|StartReactorCamera _windowcollider)
            (Variables|/Game/Blueprints/Window/WindowCollider.WindowCollider_C|SetChangedPerspective _windowcollider true)))))))

(event Input|ActionEvents|InputActionInteract
  (params (Key :type Key%20Structure :default "None"))
  (:Pressed
    (for (_array_element _array_index) (Variables|Misc|GetInteractables)
      (Variables|Misc|SetInteractableIndex _array_element)
      (switch int _array_index
        (:Default
          (CallFunction|ExampleInteraction (Variables|Misc|GetInteractableIndex)))
        (:0
          (CallFunction|ReactorInteraction (Variables|Misc|GetInteractableIndex)))
        (:1
          (CallFunction|TempInteraction (Variables|Misc|GetInteractableIndex)))
        (:2
          (CallFunction|PressureInteraction (Variables|Misc|GetInteractableIndex)))
        (:3
          (CallFunction|PowerInteraction (Variables|Misc|GetInteractableIndex)))))))

(event Input|KeyboardEvents|Left
  (params (Key :type Key%20Structure :default "None"))
  (:Pressed
    (Default|ChangeInstability (.AsReactor (Utilities|Casting|CastToReactor (Utilities|Array|Get(acopy) (Variables|Misc|GetInteractables)))) -1e+01)))

(event Input|KeyboardEvents|Right
  (params (Key :type Key%20Structure :default "None"))
  (:Pressed
    (Default|ChangeInstability (.AsReactor (Utilities|Casting|CastToReactor (Utilities|Array|Get(acopy) (Variables|Misc|GetInteractables)))) 1e+01)))

(event Input|MouseEvents|LeftMouseButton
  (params (Key :type Key%20Structure :default "None"))
  (:Pressed
    (bind _outactors (Actor|GetAllActorsOfClass "/Game/Blueprints/Tasks/TaskMaster/TaskMaster.TaskMaster_C"))
    (for _array_element _outactors
      (Class|WidgetInteractionComponent|PressPointerKey (Variables|/Game/Blueprints/Tasks/TaskMaster/TaskMaster.TaskMaster_C|GetWidgetInteraction _array_element) "LeftMouseButton")))
  (:Released
    (bind _outactors_2 (Actor|GetAllActorsOfClass "/Game/Blueprints/Tasks/TaskMaster/TaskMaster.TaskMaster_C"))
    (for _array_element_2 _outactors_2
      (Class|WidgetInteractionComponent|ReleasePointerKey (Variables|/Game/Blueprints/Tasks/TaskMaster/TaskMaster.TaskMaster_C|GetWidgetInteraction _array_element_2) "LeftMouseButton"))))

(fn ConstructionScript)