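; ExampleTask1 is a template task Blueprint that drains power while its task is left unfixed, with numbered notes marking where to customize it.
; On BeginPlay it starts a looping timer, then casts the interface widget to ExampleTaskUI1 and sets itself as that UI's parent task.
; Each timer tick shows the indicator and lowers power until TaskFixed is set.
; CompleteTask sets that flag and hides the indicator without calling the parent implementation.
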(event Custom|CustomEvent
  (if (Variables|Default|GetTaskFixed)
    (Rendering|SetVisibility (Variables|Default|GetIndicator) false false)
    (else
      ;[0.07292 0.07292 0.07292] 6. Decide what to change is we don't do the task
      (CallFunction|ChangePower -0.1)
      (Rendering|SetVisibility (Variables|Default|GetIndicator) true false))))

(event Collision|EventActorBeginOverlap
  (params (OtherActor :type Actor%20Object%20Reference)))

(event EventTick
  (params (DeltaSeconds :type Float%20%28single-precision%29)))

(event EventBeginPlay
  (bind _output_get (Variables|Default|SetMainInterface (UserInterface|GetUserWidgetObject (Variables|Default|GetInterface))))
  (Utilities|Time|SetTimerbyEvent (delegate Custom|CustomEvent) 5.0 true)
  ;[0.07292 0.07292 0.07292] 5. Change the cast to the correct UI. then change "Interface" to correct UI (top left)
  (bind _asexample_task_ui1 (Utilities|Casting|CastToExampleTaskUI1 _output_get))
  (Variables|/Game/Blueprints/Tasks/ExampleTaskUI1.ExampleTaskUI1_C|SetParentTask _asexample_task_ui1 self))

(fn ConstructionScript
  (|CallParentFunction))

(fn CompleteTask
  (Variables|Default|SetTaskFixed true)
  (Rendering|SetVisibility (Variables|Default|GetIndicator) false false))