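; ExampleTask2 is a template task Blueprint that penalizes pressure while the task remains unfixed.
; On BeginPlay it gets the widget from its Interface component, casts it to ExampleTaskUI2 and registers itself as ParentTask.
; A looping timer repeatedly lowers pressure and shows the Indicator until TaskFixed is set.
; CompleteTask sets that flag and hides the Indicator; numbered comments mark the parts to customize.
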(event Custom|CustomEvent
  (if (Variables|Default|GetTaskFixed)
    (Rendering|SetVisibility (Variables|Default|GetIndicator) false false)
    (else
      ;[0.07292 0.07292 0.07292] 6. Decide what to change is we don't do the task
      (CallFunction|ChangePressure -1.0)
      (Rendering|SetVisibility (Variables|Default|GetIndicator) true false))))

(event Collision|EventActorBeginOverlap
  (params (OtherActor :type Actor%20Object%20Reference)))

(event EventTick
  (params (DeltaSeconds :type Float%20%28single-precision%29)))

(event EventBeginPlay
  (bind _output_get (Variables|Default|SetMainInterface (UserInterface|GetUserWidgetObject (Variables|Default|GetInterface))))
  (Utilities|Time|SetTimerbyEvent (delegate Custom|CustomEvent) 5.0 true)
  ;[0.07292 0.07292 0.07292] 5. Change the cast to the correct UI. then change "Interface" to correct UI (top left)
  (bind _asexample_task_ui2 (Utilities|Casting|CastToExampleTaskUI2 _output_get))
  (Variables|/Game/Blueprints/Tasks/ExampleTaskUI2.ExampleTaskUI2_C|SetParentTask _asexample_task_ui2 self))

(fn ConstructionScript
  (|CallParentFunction))

(fn CompleteTask
  (Variables|Default|SetTaskFixed true)
  (Rendering|SetVisibility (Variables|Default|GetIndicator) false false))