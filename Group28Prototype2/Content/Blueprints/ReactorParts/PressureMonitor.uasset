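; Reactor pressure monitor actor that hosts a PressureState screen widget and gives the player a close-up view of it.
; Tick derives its Pressure from the widget's ActualB percent plus the widget's Pressure, while ChangePressure adds an amount to the widget's value.
; While the trigger is overlapped, ToggleObject blends the camera to the monitor or back to the first WindowCam-tagged actor.
; SetPressure is an empty stub.
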(event OnComponentBeginOverlap(PlayerTrigger)
  (params (OverlappedComponent :type Primitive%20Component%20Object%20Reference) (OtherActor :type Actor%20Object%20Reference) (OtherComp :type Primitive%20Component%20Object%20Reference) (OtherBodyIndex :type Integer) (bFromSweep :type Boolean) (SweepResult :type Hit%20Result%20Structure%20%28by%20ref%29))
  (Variables|Default|SetOverlapped true))

(event OnComponentEndOverlap(PlayerTrigger)
  (params (OverlappedComponent :type Primitive%20Component%20Object%20Reference) (OtherActor :type Actor%20Object%20Reference) (OtherComp :type Primitive%20Component%20Object%20Reference) (OtherBodyIndex :type Integer))
  (Variables|Default|SetOverlapped false))

(event EventToggleObject
  (params (State :type Boolean%20%28by%20ref%29))
  (if (Variables|Default|GetOverlapped)
    (if State
      (Game|Player|SetViewTargetwithBlend (Game|GetPlayerController 0) self 1.0 "VTBlend_EaseInOut" 1.0 true)
      (elif (not State)
        (bind _outactors (Actor|GetAllActorswithTag "WindowCam"))
        (Game|Player|SetViewTargetwithBlend (Game|GetPlayerController 0) (Utilities|Array|Get(acopy) _outactors) 1.0 "VTBlend_EaseInOut" 1.0 true)))))

(event EventTick
  (params (DeltaSeconds :type Float%20%28single-precision%29))
  (bind _pressureinterface (Variables|Default|GetPressureInterface))
  (Variables|Default|SetPressure (+ (Variables|/Script/UMG.ProgressBar|GetPercent (Variables|/Game/UI/PressureState.PressureState_C|GetActualB _pressureinterface)) (Variables|/Game/UI/PressureState.PressureState_C|GetPressure _pressureinterface))))

(event EventBeginPlay
  (Variables|Default|SetPressureInterface (.AsPressure%20State (Utilities|Casting|CastToPressureState (UserInterface|GetUserWidgetObject (Variables|Default|GetInterface)))))
  (Variables|Default|SetPressure (+ (Variables|Default|GetPressure) 1e+01)))

(fn ConstructionScript)

(fn ChangePressure
  (params (Amount :type Float%20%28single-precision%29))
  (bind _pressureinterface (Variables|Default|GetPressureInterface))
  (Variables|/Game/UI/PressureState.PressureState_C|SetPressure _pressureinterface (+ Amount (Variables|/Game/UI/PressureState.PressureState_C|GetPressure _pressureinterface))))

(fn SetPressure)