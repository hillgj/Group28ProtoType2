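; Reactor actor that tracks an instability value through its ReactorState widget and acts as a camera station for the player.
; Each tick it sets Instability to the widget's ActualB percent plus the widget's Instability, which ChangeInstability adjusts.
; While PlayerTrigger is overlapped, ToggleObject blends the player's view to the reactor, or back to the actor tagged WindowCam.
; SetStability is an empty stub.
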(event OnComponentBeginOverlap(PlayerTrigger)
  (params (OverlappedComponent :type Primitive%20Component%20Object%20Reference) (OtherActor :type Actor%20Object%20Reference) (OtherComp :type Primitive%20Component%20Object%20Reference) (OtherBodyIndex :type Integer) (bFromSweep :type Boolean) (SweepResult :type Hit%20Result%20Structure%20%28by%20ref%29))
  (Variables|Default|SetOverlapped true))

(event OnComponentEndOverlap(PlayerTrigger)
  (params (OverlappedComponent :type Primitive%20Component%20Object%20Reference) (OtherActor :type Actor%20Object%20Reference) (OtherComp :type Primitive%20Component%20Object%20Reference) (OtherBodyIndex :type Integer))
  (Variables|Default|SetOverlapped false))

(event EventTick
  (params (DeltaSeconds :type Float%20%28single-precision%29))
  (bind _reactorinterface (Variables|Default|GetReactorInterface))
  (Variables|Default|SetInstability (+ (Variables|/Script/UMG.ProgressBar|GetPercent (Variables|/Game/UI/ReactorState.ReactorState_C|GetActualB _reactorinterface)) (Variables|/Game/UI/ReactorState.ReactorState_C|GetInstability _reactorinterface))))

(event EventToggleObject
  (params (State :type Boolean%20%28by%20ref%29))
  (if (Variables|Default|GetOverlapped)
    (if State
      (Game|Player|SetViewTargetwithBlend (Game|GetPlayerController 0) self 1.0 "VTBlend_EaseInOut" 1.0 true)
      (elif (not State)
        (bind _outactors (Actor|GetAllActorswithTag "WindowCam"))
        (Game|Player|SetViewTargetwithBlend (Game|GetPlayerController 0) (Utilities|Array|Get(acopy) _outactors) 1.0 "VTBlend_EaseInOut" 1.0 true)))))

(event EventBeginPlay
  (Variables|Default|SetReactorInterface (.AsReactor%20State (Utilities|Casting|CastToReactorState (UserInterface|GetUserWidgetObject (Variables|Default|GetInterface)))))
  (Variables|Default|SetInstability (+ (Variables|Default|GetInstability) 1e+01)))

(fn ConstructionScript)

(fn ChangeInstability
  (params (Amount :type Float%20%28single-precision%29))
  (bind _reactorinterface (Variables|Default|GetReactorInterface))
  (Variables|/Game/UI/ReactorState.ReactorState_C|SetInstability _reactorinterface (+ Amount (Variables|/Game/UI/ReactorState.ReactorState_C|GetInstability _reactorinterface))))

(fn SetStability)