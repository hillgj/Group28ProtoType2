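; Reactor temperature monitor actor that the player can switch the camera to while inside its trigger.
; Temperature lives on a TempState widget in the Interface component; Tick sums it with the ActualB percent into the actor's Temperature, and ChangeTemperature adds to the widget's value.
; ToggleObject, gated by overlap, blends the view to this actor or back to the WindowCam-tagged actor.
; SetTemp is an empty stub.
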(event OnComponentBeginOverlap(PlayerTrigger)
  (params (OverlappedComponent :type Primitive%20Component%20Object%20Reference) (OtherActor :type Actor%20Object%20Reference) (OtherComp :type Primitive%20Component%20Object%20Reference) (OtherBodyIndex :type Integer) (bFromSweep :type Boolean) (SweepResult :type Hit%20Result%20Structure%20%28by%20ref%29))
  (Variables|Default|SetOverlapped true))

(event OnComponentEndOverlap(PlayerTrigger)
  (params (OverlappedComponent :type Primitive%20Component%20Object%20Reference) (OtherActor :type Actor%20Object%20Reference) (OtherComp :type Primitive%20Component%20Object%20Reference) (OtherBodyIndex :type Integer))
  (Variables|Default|SetOverlapped false))

(event EventToggleObject
  (params (State :type Boolean%20%28by%20ref%29))
  (if (Variables|Default|GetOverlapped)
    (if State
      (Game|Player|SetViewTargetwithBlend (Game|GetPlayerController 0) self 1.0 "VTBlend_EaseInOut" 1.0 true)
      (elif (not State)
        (bind _outactors (Actor|GetAllActorswithTag "WindowCam"))
        (Game|Player|SetViewTargetwithBlend (Game|GetPlayerController 0) (Utilities|Array|Get(acopy) _outactors) 1.0 "VTBlend_EaseInOut" 1.0 true)))))

(event EventTick
  (params (DeltaSeconds :type Float%20%28single-precision%29))
  (bind _tempinterface (Variables|Default|GetTempInterface))
  (Variables|Default|SetTemperature (+ (Variables|/Script/UMG.ProgressBar|GetPercent (Variables|/Game/UI/TempState.TempState_C|GetActualB _tempinterface)) (Variables|/Game/UI/TempState.TempState_C|GetTemperature _tempinterface))))

(event EventBeginPlay
  (Variables|Default|SetTempInterface (.AsTemp%20State (Utilities|Casting|CastToTempState (UserInterface|GetUserWidgetObject (Variables|Default|GetInterface)))))
  (Variables|Default|SetTemperature (+ (Variables|Default|GetTemperature) 1e+01)))

(fn ConstructionScript)

(fn ChangeTemperature
  (params (Amount :type Float%20%28single-precision%29))
  (bind _tempinterface (Variables|Default|GetTempInterface))
  (Variables|/Game/UI/TempState.TempState_C|SetTemperature _tempinterface (+ Amount (Variables|/Game/UI/TempState.TempState_C|GetTemperature _tempinterface))))

(fn SetTemp)